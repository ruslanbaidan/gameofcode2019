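; BP_FloorTile_END2 is a runner floor tile that ends the game.
; Its construction script randomly adds child-actor coins within CoinArea or a blocker at one of three spawn points, plus another blocker once RunGameMode's Time passes a threshold.
; When any actor leaves EndTrigger it shows the EndText widget; if that actor is the RunCharacter, it destroys it and quits after a short delay.
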(event `self.EndTrigger.OnComponentEndOverlap`
  (params (OverlappedComponent :type "PrimitiveComponent Object Reference") (OtherActor :type "Actor Object Reference") (OtherComp :type "PrimitiveComponent Object Reference") (OtherBodyIndex :type Integer))
  (bind _returnvalue (`|CreateWidget` "/Game/ItemPickup/EndText.EndText_C"))
  (`UserWidget.AddToViewport` _returnvalue 0)
  (bind _asrun_character (cast `/Game/ThirdPersonBP/Blueprints/RunCharacter` OtherActor))
  (`self.K2_DestroyActor` _asrun_character)
  (`KismetSystemLibrary.Delay` 4.0)
  (`KismetSystemLibrary.QuitGame` null "Quit"))

(fn `GetAttachTransform`)

(fn `SetSpawmPoints`
  (set `self.SpawnPoints` (`|MakeArray` (`SceneComponent.GetRelativeTransform` (`self.Spawm_Point_R`)) (`SceneComponent.GetRelativeTransform` (`self.Spawm_Point_L`)) (`SceneComponent.GetRelativeTransform` (`self.Spawm_Point`)))))

(fn `spawm_coins`
  (bind _coinarea (`self.CoinArea`))
  (for _ (range 4)
    (`AddComponent|NODE_AddChildActorComponent-0` :`RelativeTransform` (`KismetMathLibrary.Conv_VectorToTransform` (`KismetMathLibrary.RandomPointInBoundingBox` (`SceneComponent.RelativeLocation` _coinarea) (`BoxComponent.BoxExtent` _coinarea))))))

(fn `SpawmBlocker`
  (bind _spawnpoints (`self.SpawnPoints`))
  (`AddComponent|NODE_AddChildActorComponent-1` :`RelativeTransform` (`|GetArrayItem` _spawnpoints (`KismetMathLibrary.RandomIntegerInRange` 0 (`KismetArrayLibrary.Array_LastIndex` _spawnpoints)))))

(fn `UserConstructionScript`
  (`self.SetSpawmPoints`)
  (switch `int` (`KismetMathLibrary.RandomIntegerInRange` 0 1)
    (:`Default`
      (`self.SpawmBlocker` :!label _label)
      (bind _asrun_game_mode (cast `/Game/ThirdPersonBP/Blueprints/RunGameMode` (`GameplayStatics.GetGameMode`)))
      (if (> (`/Game/ThirdPersonBP/Blueprints/RunGameMode.Time` _asrun_game_mode) 10)
        (`self.SpawmBlocker`)))
    (:`0`
      (goto _label))
    (:`1`
      (`self.spawm_coins`))))